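; BPC_DamageSystem is a damage component that tracks health, death, blocking, invincibility and interruptibility.
; TakeDamage runs a CanBeDamaged macro that routes each DamageInfo to blocked, damage or no-damage, with per-hit overrides for invincibility, blocking and interruption.
; Results fire OnBlocked with parry eligibility, OnDeath, or OnDamageResponse for interrupting hits.
; Heal returns health plus the amount, clamped to MaxHealth, without storing it.
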(fn `Heal`
  (params (Amount :type "Float (double-precision)"))
  (returns (`New Health` :type "Float (double-precision)"))
  (if (not (`self.isDead?`))
    (return (`KismetMathLibrary.FClamp` (+ (`self.Health`) Amount) 0.0 (`self.MaxHealth`)))))

(fn `TakeDamage`
  (params (DamageInfo :type "/Game/DamageSystem/S_DamageInfo Structure"))
  (returns (`was Damaged?` :type Boolean))
  (bind (_amount _damagetype _damageresponse _shoulddamageinvincible_ _canbeblocked_ _canbeparried_ _forceinterrupt_) (break `/Game/DamageSystem/S_DamageInfo` DamageInfo))
  (`self.Can Be Damaged?` _shoulddamageinvincible_ _canbeblocked_
    (:`Blocked Damage`
      (`self.OnBlocked` _canbeparried_)
      (return false))
    (:`Do Damage`
      (bind _output_get (set `self.Health` (- (`self.Health`) _amount)))
      (if (<= _output_get 0.0)
        (set `self.isDead?` true)
        (`self.OnDeath`)
        (return true)
        (elif (or (`self.isInterruptible?`) _forceinterrupt_)
          (`self.OnDamageResponse` _damageresponse)
          (return true))))
    (:`No Damage`
      (return false))))