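; BP_Platform is a platform that the knight can drop through by pressing S, which turns off the Cube's collision.
; Overlap of BP_Knight with the Box restores query-and-physics collision and enables the platform's input for player 0.
; The Cube's own overlap does the same but passes no player controller.
; End overlap does nothing, and the logic to disable input is disconnected, so input is never turned off.
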(event `Key|S`
  (params (Key :type "Key Structure"))
  (:`Pressed`
    (`PrimitiveComponent.SetCollisionEnabled` (`self.Cube`) "NoCollision")))

(event `self.Box.OnComponentEndOverlap`
  (params (OverlappedComponent :type "PrimitiveComponent Object Reference") (OtherActor :type "Actor Object Reference") (OtherComp :type "PrimitiveComponent Object Reference") (OtherBodyIndex :type Integer)))

(event `self.Box.OnComponentBeginOverlap`
  (params (OverlappedComponent :type "PrimitiveComponent Object Reference") (OtherActor :type "Actor Object Reference") (OtherComp :type "PrimitiveComponent Object Reference") (OtherBodyIndex :type Integer) (bFromSweep :type Boolean) (SweepResult :type "HitResult Structure (by ref)"))
  (cast `/Game/PaperZD/BP_Knight` OtherActor)
  (`PrimitiveComponent.SetCollisionEnabled` (`self.Cube`) "QueryAndPhysics")
  (`self.EnableInput` (`GameplayStatics.GetPlayerController` 0)))

(event `self.Cube.OnComponentBeginOverlap`
  (params (OverlappedComponent :type "PrimitiveComponent Object Reference") (OtherActor :type "Actor Object Reference") (OtherComp :type "PrimitiveComponent Object Reference") (OtherBodyIndex :type Integer) (bFromSweep :type Boolean) (SweepResult :type "HitResult Structure (by ref)"))
  (cast `/Game/PaperZD/BP_Knight` OtherActor)
  (`PrimitiveComponent.SetCollisionEnabled` (`self.Cube`) "QueryAndPhysics")
  (`self.EnableInput` null))

(fn `UserConstructionScript`)