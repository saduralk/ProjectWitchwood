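; BP_FlipbookChangeTest is a test actor that starts dialogue with the knight and can switch its Paper2D flipbook.
; Its Box trigger enables input while BP_Knight overlaps, so E starts the conversation and key 6 sets the Run flipbook.
; With Cutscene set, overlap starts the conversation automatically.
; DialogueHandler runs behind a RunningCutscene guard, blocks player movement and shows a Dialogue_HUD fed DialogueInfo and this actor as Speaker.
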(event `StartConversation`
  (`self.Dialogue Handler`))

(event `Key|Six`
  (params (Key :type "Key Structure"))
  (:`Pressed`
    (`PaperFlipbookComponent.SetFlipbook` (`self.PaperFlipbook`) "/Game/Sprites_Adventurer/Run/Run.Run")))

(event `Key|E`
  (params (Key :type "Key Structure"))
  (:`Pressed`
    (`self.StartConversation`)))

(event `self.Box.OnComponentBeginOverlap`
  (params (OverlappedComponent :type "PrimitiveComponent Object Reference") (OtherActor :type "Actor Object Reference") (OtherComp :type "PrimitiveComponent Object Reference") (OtherBodyIndex :type Integer) (bFromSweep :type Boolean) (SweepResult :type "HitResult Structure (by ref)"))
  (cast `/Game/PaperZD/BP_Knight` OtherActor)
  (`self.EnableInput` (`GameplayStatics.GetPlayerController` 0))
  (if (`self.cutscene?`)
    (`self.StartConversation`)))

(event `self.Box.OnComponentEndOverlap`
  (params (OverlappedComponent :type "PrimitiveComponent Object Reference") (OtherActor :type "Actor Object Reference") (OtherComp :type "PrimitiveComponent Object Reference") (OtherBodyIndex :type Integer))
  (cast `/Game/PaperZD/BP_Knight` OtherActor)
  (`self.DisableInput` (`GameplayStatics.GetPlayerController` 0)))

(fn `UserConstructionScript`)