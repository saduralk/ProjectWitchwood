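; BP_DialogueTrigger is a trigger volume that opens dialogue when BP_Knight is inside its box.
; Box overlaps toggle player input so E can call DialogueHandler, while the Cutscene flag auto-starts the conversation once on first qualifying entry.
; DialogueHandler uses RunningCutscene to block repeat starts, then creates a Dialogue_HUD widget with DialogueInfo and itself as Speaker, adds it to the viewport and stores a reference.
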(event `Key|E`
  (params (Key :type "Key Structure"))
  (:`Pressed`
    (`self.Dialogue Handler`)))

(event `self.Box.OnComponentBeginOverlap`
  (params (OverlappedComponent :type "PrimitiveComponent Object Reference") (OtherActor :type "Actor Object Reference") (OtherComp :type "PrimitiveComponent Object Reference") (OtherBodyIndex :type Integer) (bFromSweep :type Boolean) (SweepResult :type "HitResult Structure (by ref)"))
  (cast `/Game/PaperZD/BP_Knight` OtherActor)
  (`self.EnableInput` (`GameplayStatics.GetPlayerController` 0))
  ;[1 1 1] If 'Cutscene' var = true, automatically start conversation
  (if (`self.Cutscene?`)
    (`/Engine/EditorBlueprintResources/StandardMacros.DoOnce` false
      (:`Completed`
        (`self.Dialogue Handler`)))))

(event `self.Box.OnComponentEndOverlap`
  (params (OverlappedComponent :type "PrimitiveComponent Object Reference") (OtherActor :type "Actor Object Reference") (OtherComp :type "PrimitiveComponent Object Reference") (OtherBodyIndex :type Integer))
  (cast `/Game/PaperZD/BP_Knight` OtherActor)
  (`self.DisableInput` (`GameplayStatics.GetPlayerController` 0)))

(fn `UserConstructionScript`)